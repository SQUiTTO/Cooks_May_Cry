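; Player character Blueprint that handles movement, punching, interaction and menu pointer input.
; Enhanced Input drives camera-relative movement, a double jump via DoN that resets on landing, and Sprint, which becomes a forward launch when airborne.
; Punch cycles a combo counter and flags presses made mid-attack; its montage call is disconnected.
; E messages the first overlapping InteractInterface actor, while mouse clicks and scrolling feed a WidgetInteraction component when the menu is open.
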(event Custom|AttackEnding
  (Variables|Default|SetIsAttacking false))

(event Custom|Release%20Pointer
  (Class|WidgetInteractionComponent|ReleasePointerKey (Variables|Default|GetWidgetInteraction) "LeftMouseButton"))

(event Custom|Press%20Pointer
  (Class|WidgetInteractionComponent|PressPointerKey (Variables|Default|GetWidgetInteraction) "LeftMouseButton"))

(event Custom|WheelDown
  (Class|WidgetInteractionComponent|ScrollWheel (Variables|Default|GetWidgetInteraction) -1.0))

(event Custom|WheelUp
  (Class|WidgetInteractionComponent|ScrollWheel (Variables|Default|GetWidgetInteraction) 1.0))

(event Custom|ResetCam
  (bind _returnvalue (Pawn|GetController))
  (bind _mesh (Variables|Character|GetMesh))
  (bind _returnvalue_2 (Transformation|GetWorldRotation _mesh))
  (bind _returnvalue_3 (Pawn|GetControlRotation _returnvalue :!class /Script/Engine.Controller))
  (bind _returnvalue_4 (Math|Rotator|Delta(Rotator) _returnvalue_2 _returnvalue_3))
  (bind (_roll _pitch _yaw) (Math|Rotator|BreakRotator _returnvalue_4))
  (Pawn|Input|AddControllerYawInput _yaw)
  (Pawn|Input|AddControllerPitchInput _pitch)
  (Pawn|Input|AddControllerRollInput _roll))

(event Input|EnhancedActionEvents|EnhancedInputActionMoveForward_CC
  (params (ActionValue :type Float%20%28double-precision%29) (ElapsedSeconds :type Float%20%28double-precision%29) (TriggeredSeconds :type Float%20%28double-precision%29) (InputAction :type Input%20Action%20Object%20Reference :default "/Game/Inputs/MoveForward_CC.MoveForward_CC"))
  (:Triggered
    (Pawn|Input|AddMovementInput (Math|Vector|GetForwardVector (Math|Rotator|MakeRotator 0.0 0.0 (.Yaw (Math|Rotator|BreakRotator (Pawn|GetControlRotation :!class /Script/Engine.Pawn))))) ActionValue false)))

(event Input|EnhancedActionEvents|EnhancedInputActionMoveRight_CC
  (params (ActionValue :type Float%20%28double-precision%29) (ElapsedSeconds :type Float%20%28double-precision%29) (TriggeredSeconds :type Float%20%28double-precision%29) (InputAction :type Input%20Action%20Object%20Reference :default "/Game/Inputs/MoveRight_CC.MoveRight_CC"))
  (:Triggered
    (Pawn|Input|AddMovementInput (Math|Vector|GetRightVector (Math|Rotator|MakeRotator 0.0 0.0 (.Yaw (Math|Rotator|BreakRotator (Pawn|GetControlRotation :!class /Script/Engine.Pawn))))) ActionValue false)))

(event Input|EnhancedActionEvents|EnhancedInputActionTurnRight_CC
  (params (ActionValue :type Float%20%28double-precision%29) (ElapsedSeconds :type Float%20%28double-precision%29) (TriggeredSeconds :type Float%20%28double-precision%29) (InputAction :type Input%20Action%20Object%20Reference :default "/Game/Inputs/TurnRight_CC.TurnRight_CC"))
  (:Triggered
    (Pawn|Input|AddControllerYawInput ActionValue)))

(event Input|EnhancedActionEvents|EnhancedInputActionLookUp_CC
  (params (ActionValue :type Float%20%28double-precision%29) (ElapsedSeconds :type Float%20%28double-precision%29) (TriggeredSeconds :type Float%20%28double-precision%29) (InputAction :type Input%20Action%20Object%20Reference :default "/Game/Inputs/LookUp_CC.LookUp_CC"))
  (:Triggered
    (Pawn|Input|AddControllerPitchInput ActionValue)))

(event Input|EnhancedActionEvents|EnhancedInputActionJump_CC
  (params (ActionValue :type Boolean) (ElapsedSeconds :type Float%20%28double-precision%29) (TriggeredSeconds :type Float%20%28double-precision%29) (InputAction :type Input%20Action%20Object%20Reference :default "/Game/Inputs/Jump_CC.Jump_CC"))
  (:Started
    (Utilities|FlowControl|DoN 2
      (:Exit
        (Character|LaunchCharacter (Math|Vector|MakeVector 0.0 0.0 (Variables|/Script/Engine.CharacterMovementComponent|GetJumpZVelocity (Variables|Character|GetCharacterMovement))) false true)
        (Variables|Default|SetIsJumping true)))))

(event Input|EnhancedActionEvents|EnhancedInputActionSprint_CC
  (params (ActionValue :type Boolean) (ElapsedSeconds :type Float%20%28double-precision%29) (TriggeredSeconds :type Float%20%28double-precision%29) (InputAction :type Input%20Action%20Object%20Reference :default "/Game/Inputs/Sprint_CC.Sprint_CC"))
  (:Triggered
    (if (Variables|Default|GetinAir?)
      (goto _label Reset)))
  (:Started
    (if (Variables|Default|GetinAir?)
      (Utilities|FlowControl|DoOnce false :!label _label
        (:Completed
          (Character|LaunchCharacter (* (Math|Vector|GetForwardVector (Variables|Collision|GetCapsuleComponent)) 1.1e+03) true false)))
      (else
        (Variables|Default|SetIsSprinting true)
        (Variables|/Script/Engine.CharacterMovementComponent|SetMaxWalkSpeed (Variables|Character|GetCharacterMovement) 725.0))))
  (:Completed
    (Variables|Default|SetIsSprinting false)
    (Variables|/Script/Engine.CharacterMovementComponent|SetMaxWalkSpeed (Variables|Character|GetCharacterMovement) 2.5e+02)))

(event Input|EnhancedActionEvents|EnhancedInputActionPunch_CC
  (params (ActionValue :type Boolean) (ElapsedSeconds :type Float%20%28double-precision%29) (TriggeredSeconds :type Float%20%28double-precision%29) (InputAction :type Input%20Action%20Object%20Reference :default "/Game/Inputs/Punch_CC.Punch_CC"))
  (:Started
    (if (Variables|Default|GetIsAttacking)
      (Variables|Default|SetSaveAttack true)
      (else
        (Variables|Default|SetIsAttacking true)
        (Variables|Default|SetSet%20Damage 2.5e+02)
        (switch int (Variables|Default|GetAttackCount)
          (:0
            (Variables|Default|SetAttackCount 1))
          (:1
            (Variables|Default|SetAttackCount 2))
          (:2
            (Variables|Default|SetAttackCount 3))
          (:3
            (Variables|Default|SetAttackCount 0)))))))

(event EventTick
  (params (DeltaSeconds :type Float%20%28single-precision%29))
  (bind _output_get (Variables|Default|SetinAir? (AI|Components|NavMovement|IsFalling (Variables|Character|GetCharacterMovement))))
  (if _output_get
    _))

(event EventOnLanded
  (params (Hit :type Hit%20Result%20Structure%20%28by%20ref%29))
  (Variables|Default|SetIsJumping false)
  (Utilities|FlowControl|DoN 2) ; enters at Reset
)

(event EventPossessed
  (params (NewController :type Controller%20Object%20Reference))
  (bind _asplayer_controller (Utilities|Casting|CastToPlayerController NewController))
  (bind _output_get (Variables|Default|SetPlayerController _asplayer_controller))
  (Input|AddMappingContext (PlayerController|LocalPlayerSubsystems|GetEnhancedInputLocalPlayerSubsystem _output_get) "/Game/Inputs/PlayerInput_Context.PlayerInput_Context" 0 "(bIgnoreAllPressedKeysUntilRelease=True,bForceImmediately=False)"))

(event Input|KeyboardEvents|E
  (params (Key :type Key%20Structure :default "None"))
  (:Pressed
    (bind _array_element (Utilities|Array|ForEachLoopwithBreak (Collision|GetOverlappingActors 0 :!class /Script/Engine.Actor) :!label _label)
      (:LoopBody
        (if (Utilities|DoesObjectImplementInterface _array_element "/Game/Levels/TestLevels/InteractInterface.InteractInterface_C")
          (Class|InteractInterface|Interact(Message) _array_element)
          (goto _label Break))))))

(event Input|MouseEvents|LeftMouseButton
  (params (Key :type Key%20Structure :default "None"))
  (bind _ismenuopen (Variables|Default|GetIsMenuOpen))
  (:Pressed
    (if _ismenuopen
      (CallFunction|PressPointer)))
  (:Released
    (if _ismenuopen
      (CallFunction|ReleasePointer))))

(event Input|MouseEvents|MouseWheelDown
  (params (Key :type Key%20Structure :default "None"))
  (:Pressed
    (if (Variables|Default|GetIsMenuOpen)
      (CallFunction|WheelDown))))

(event Input|MouseEvents|MouseWheelUp
  (params (Key :type Key%20Structure :default "None"))
  (:Pressed
    (if (Variables|Default|GetIsMenuOpen)
      (CallFunction|WheelUp))))

(fn ConstructionScript)